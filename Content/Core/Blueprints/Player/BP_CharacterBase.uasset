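; BP_CharacterBase is a player character Blueprint that handles movement, look, jump and interaction through Enhanced Input.
; On BeginPlay, only a locally controlled instance adds IMC_Default via its MyPlayerControllerBase's input subsystem, printing debug messages when a check fails.
; Movement follows control-rotation yaw, look feeds controller yaw and pitch, and interaction calls TryInteract, which is defined outside these graphs.
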(event `EnhancedInput|/Game/Systems/Input/IA_Interaction`
  (params (ActionValue :type Boolean) (ElapsedSeconds :type "Float (double-precision)") (TriggeredSeconds :type "Float (double-precision)") (InputAction :type "InputAction Object Reference" :default "/Game/Systems/Input/IA_Interaction.IA_Interaction"))
  (:`Started`
    (`self.TryInteract`)))

(event `EnhancedInput|/Game/Systems/Input/IA_Jump`
  (params (ActionValue :type Boolean) (ElapsedSeconds :type "Float (double-precision)") (TriggeredSeconds :type "Float (double-precision)") (InputAction :type "InputAction Object Reference" :default "/Game/Systems/Input/IA_Jump.IA_Jump"))
  (:`Started`
    (`self.Jump`))
  (:`Completed`
    (`self.StopJumping`)))

(event `EnhancedInput|/Game/Systems/Input/IA_Look`
  (params (ActionValue :type "Vector2D Structure") (ElapsedSeconds :type "Float (double-precision)") (TriggeredSeconds :type "Float (double-precision)") (InputAction :type "InputAction Object Reference" :default "/Game/Systems/Input/IA_Look.IA_Look"))
  (bind (_x _y) (`KismetMathLibrary.BreakVector2D` ActionValue))
  (:`Triggered`
    (`|ExecutionSequence`
      (:`then_0`
        (`self.AddControllerYawInput` _x))
      (:`then_1`
        (`self.AddControllerPitchInput` _y)))))

(event `EnhancedInput|/Game/Systems/Input/IA_Move`
  (params (ActionValue :type "Vector2D Structure") (ElapsedSeconds :type "Float (double-precision)") (TriggeredSeconds :type "Float (double-precision)") (InputAction :type "InputAction Object Reference" :default "/Game/Systems/Input/IA_Move.IA_Move"))
  (bind (_x _y) (`KismetMathLibrary.BreakVector2D` ActionValue))
  (bind _returnvalue (`KismetMathLibrary.MakeRotator` 0.0 0.0 (.yaw (`self.GetControlRotation`))))
  (:`Triggered`
    (`|ExecutionSequence`
      (:`then_0`
        (`self.AddMovementInput` (`KismetMathLibrary.GetRightVector` _returnvalue) _x))
      (:`then_1`
        (`self.AddMovementInput` (`KismetMathLibrary.GetForwardVector` _returnvalue) _y)))))

(event `self.ReceiveBeginPlay`
  (bind _returnvalue (`self.GetController`))
  (if (`self.IsLocallyControlled`)
    (`/Engine/EditorBlueprintResources/StandardMacros.IsValid` _returnvalue
      (:`Is Valid`
        (bind _asmy_player_controller_base (cast `MyPlayerControllerBase` _returnvalue)
          (:`then`
            (bind _returnvalue_2 (pcsubsystem `EnhancedInputLocalPlayerSubsystem` _asmy_player_controller_base))
            (`/Engine/EditorBlueprintResources/StandardMacros.IsValid` _returnvalue_2
              (:`Is Valid`
                (`EnhancedInputSubsystemInterface.AddMappingContext` _returnvalue_2 "/Game/Systems/Input/IMC_Default.IMC_Default" 0 (struct)))
              (:`Is Not Valid`
                (`KismetSystemLibrary.PrintString` "Invalid"))))
          (:`CastFailed`
            (`KismetSystemLibrary.PrintString` "Cast Failed"))))
      (:`Is Not Valid`
        (`KismetSystemLibrary.PrintString` "Start Invalid")))
    (else
      (`KismetSystemLibrary.PrintString` "This isn't locally controlled"))))

(fn `UserConstructionScript`)